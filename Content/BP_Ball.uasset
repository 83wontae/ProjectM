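; BP_Ball is a physics projectile that knocks back BP_CharacterM characters it hits.
; On BeginPlay it launches its Sphere along the actor's forward vector, scaled by an Impulse variable, and destroys itself after a short delay.
; On a Sphere hit with that character, it prints the normal impulse for debugging and applies its negation to CharacterMovement, transferring the physics collision force to the character.
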(event OnComponentHit(Sphere)
  (params (HitComponent :type Primitive%20Component%20Object%20Reference) (OtherActor :type Actor%20Object%20Reference) (OtherComp :type Primitive%20Component%20Object%20Reference) (NormalImpulse :type Vector :default "0, 0, 0") (Hit :type Hit%20Result%20Structure%20%28by%20ref%29))
  (bind _asbp_character_m (Utilities|Casting|CastToBP_CharacterM OtherActor))
  (Development|PrintString (Utilities|String|Append "Hit Character - " (Utilities|GetDisplayName _asbp_character_m)) false false)
  (Development|PrintString (Utilities|String|Append "Physics Linear Velocity = " (Utilities|String|ToString(Vector) NormalImpulse)))
  (Physics|AddImpulse (Variables|/Script/Engine.Character|GetCharacterMovement _asbp_character_m) (Math|Vector|NegateVector NormalImpulse) false))

(event EventBeginPlay
  (Physics|AddImpulse (Variables|Default|GetSphere) (* (Transformation|GetActorForwardVector) (Variables|Default|GetImpulse)) "None" false)
  (Utilities|FlowControl|Delay 5.0)
  (Actor|DestroyActor))

(fn ConstructionScript)